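; Notes Blueprint that checks typed keys against a target string, forming a basic typing mechanic.
; On BeginPlay it binds to the Player pawn's key-emit event and splits the current SentenceArray entry into characters.
; Each key matching the uppercased expected character is appended to LettersCorrect, advances the character index and prints the progress.
; Wrong keys leave progress unchanged, and nothing here advances to another sentence or handles completion.
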(event Custom|GetEmittedKey
  (params (KeyInputted :type String))
  (bind _output_get (Variables|Default|SetPressedKey KeyInputted))
  (if (Utilities|Enum|Equal(Enum) (Class|KismetStringLibrary|ToUpper (Utilities|Array|Get(acopy) (stale EventBeginPlay _output_get_2) (Variables|Default|GetcurrentWordIndex))) KeyInputted)
    (bind _returnstring (CallFunction|AppendString (Variables|Default|GetlettersCorrect) _output_get))
    (bind _output_get_2 (Variables|Default|SetlettersCorrect _returnstring))
    (bind _result (Math|Integer|IncrementInt (Variables|Default|GetcurrentWordIndex))
      (:%20%20
        (Variables|Default|SetcurrentWordIndex _result)
        (Development|PrintString _output_get_2)))))

(event EventBeginPlay
  (bind _asplayer (Utilities|Casting|CastToPlayer (Game|Player|GetPlayerPawn 0)))
  (EventDispatchers|BindEventtoEmitKey _asplayer (delegate Custom|GetEmittedKey))
  (bind _output_get (Variables|Default|SetcurrentWord (Utilities|Array|Get(acopy) (Variables|Default|GetsentenceArray) (Variables|Default|GetcurrentSentenceIndex))))
  (bind _output_get_2 (Variables|Default|SetcurrentWordArray (Utilities|String|GetCharacterArrayfromString _output_get))))

(fn ConstructionScript)

(fn AppendString
  (params (NewParam :type String) (NewParam1 :type String))
  (return (Utilities|String|Append NewParam NewParam1)))